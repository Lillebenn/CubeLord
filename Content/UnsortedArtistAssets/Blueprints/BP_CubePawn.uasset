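; BP_CubePawn is a launchable cube that slides across the level and attacks BP_EnemySlow actors it overlaps while moving.
; Hits launch it away along the nearest X/Y axis and magnet impulses along a given direction, with Tick driving FloatingPawnMovement until velocity reaches zero.
; A downward trace detects drops, ending any magnet, snapping to the tile below and boosting the cube down.
; Helper events control beam and trail particles.
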(event OnComponentBeginOverlap(CubeCollision)
  (params (OverlappedComponent :type Primitive%20Component%20Object%20Reference) (OtherActor :type Actor%20Object%20Reference) (OtherComp :type Primitive%20Component%20Object%20Reference) (OtherBodyIndex :type Integer) (bFromSweep :type Boolean) (SweepResult :type Hit%20Result%20Structure%20%28by%20ref%29))
  ;[1 1 1] LaunchFunctionality, TODO: Lots of hard-coding, needs to be fixed
  (if (Variables|Default|GetbCubeAboveThresholdSpeed)
    (bind _asbp_enemy_slow (Utilities|Casting|CastToBP_EnemySlow OtherActor))
    (Default|AttackReceived _asbp_enemy_slow)))

(event Custom|HitReceived
  (params (HitFromLocation :type Vector))
  (bind _returnvalue (Transformation|GetActorLocation))
  (bind _returnvalue_2 (- (Math|Vector|MakeVector (.x HitFromLocation) (.y HitFromLocation) 0.0) (Math|Vector|MakeVector (.x _returnvalue) (.y _returnvalue) 0.0)))
  (bind _returnvalue_3 (Math|Vector|Normalize _returnvalue_2))
  ;[0.3782 0.2648 1] FindClosestXYDirection
  (if (not (Variables|Default|GetbCubeLaunched))
    (bind (_outx _outy) (CallFunction|FindNearestDirection (.x _returnvalue_3) (.y _returnvalue_3)))
    (Variables|Default|SetCurrentLaunchDirection (* (Math|Vector|MakeVector (Math|Conversions|ToFloat(Integer) _outx) (Math|Conversions|ToFloat(Integer) _outy) 0.0) -1.0))
    ;[1 0 0.06404] CubeLaunch
    (CallFunction|SetCollisionObjectType true)
    (Variables|Default|SetbCubeLaunched true)))

(event Custom|SpawnEmitter
  (bind _currentlaunchdirection (Variables|Default|GetCurrentLaunchDirection))
  (bind _cubetrails (Variables|Default|GetCubeTrails))
  (bind _returnvalue (* _currentlaunchdirection -1.0))
  ;[0.4319 1 0] ParticleStuff
  (Utilities|FlowControl|DoOnce false
    (:Completed
      (Utilities|IsValid _cubetrails
        (:Is%20Valid
          (Effects|Components|ParticleSystem|SetVectorParameter _cubetrails "EmitterDirection" (Math|Vector|MakeVector (.x _returnvalue) (.y _returnvalue) 0.6))
          (Components|Activation|Activate _cubetrails true))))))

(event Custom|ResetCheckForCubeVelocity
  ;[1 0 0.06404] CubeLaunch
  (Utilities|FlowControl|DoOnce false) ; enters at Reset
)

(event Custom|MagnetImpulseReceived
  (params (inDirection :type Vector) (launchedByCharacter :type BP%20Player%20Character%20Object%20Reference))
  ;[0.3782 0.2648 1] FindClosestXYDirection
  (if (not (Variables|Default|GetbCubeLaunched))
    (bind _output_get (Variables|Default|SetLaunchedByCharacter launchedByCharacter))
    (Animation|PlayAnimMontage _output_get "/Game/Meshes/Character/Animations/MagnetActivated_Montage.MagnetActivated_Montage" 0.2 "None")
    (Variables|Default|SetCurrentLaunchDirection inDirection)
    ;[1 0 0.06404] CubeLaunch
    (CallFunction|SetCollisionObjectType true)
    (Variables|Default|SetbCubeLaunched true)))

(event Custom|ResetPosition
  (Transformation|SetActorTransform (Variables|Default|GetInitialLocation)))

(event Custom|AddDownWardForce
  (params (DeltaSeconds :type Float%20%28single-precision%29))
  (bind _returnvalue (Transformation|GetActorLocation))
  (bind _launchedbycharacter (Variables|Default|GetLaunchedByCharacter))
  (bind _outhit (Collision|LineTraceByChannel (+ _returnvalue "0, 0,-100.000000") (+ _returnvalue "0, 0,-1000.000000") "TraceTypeQuery1" false 0 "None"))
  (if (> (.distance _outhit) 199.0)
    (Variables|Default|SetbCubeLaunched false)
    (Utilities|IsValid _launchedbycharacter
      (:Is%20Valid
        (if (Variables|/Game/UnsortedArtistAssets/Blueprints/BP_PlayerCharacter.BP_PlayerCharacter_C|GetbMagnetStarted _launchedbycharacter)
          (Default|MagnetEnded (Variables|Default|GetLaunchedByCharacter))))
      (:Is%20Not%20Valid
        _))
    (Utilities|FlowControl|DoOnce false :!label _label
      (:Completed
        (Components|Movement|StopMovementImmediately (Variables|Default|GetFloatingPawnMovement))
        (bind _asbp_level_tile (Utilities|Casting|CastToBP_LevelTile (.hitactor _outhit)))
        (Transformation|SetActorLocation (Math|Vector|MakeVector (.x (Transformation|GetWorldLocation (Variables|/Game/UnsortedArtistAssets/Blueprints/BP_LevelTile.BP_LevelTile_C|GetTile _asbp_level_tile))) (.y (Transformation|GetWorldLocation (Variables|/Game/UnsortedArtistAssets/Blueprints/BP_LevelTile.BP_LevelTile_C|GetTile _asbp_level_tile))) (.z (Transformation|GetWorldLocation (Variables|Default|GetGridCollision)))) false false)
        (Utilities|FlowControl|Delay 0.3)
        (Variables|Default|SetCurrentLaunchDirection "0, 0,-1.000000")
        (Timeline|DownwardBoost Play
          (:Update
            (Class|PawnMovementComponent|AddInputVector (Variables|Default|GetFloatingPawnMovement) (* (* (Variables|Default|GetCurrentLaunchDirection) (Variables|Default|GetBaseLaunchVelocity)) (Variables|Default|GetDeltaSeconds)) true)
            (CallFunction|SetCollisionObjectType true)
            (Variables|Default|SetbCubeLaunched true)
            (Utilities|FlowControl|Delay 2.0)
            (Collision|SetCollisionResponsetoAllChannels (Variables|Default|GetGridCollision) "ECR_Block")))))
    (else
      (goto _label Reset))))

(event Custom|DespawnEmitter
  (bind _currentlaunchdirection (Variables|Default|GetCurrentLaunchDirection))
  (bind _cubetrails (Variables|Default|GetCubeTrails))
  (bind _cubetrails_2 (Variables|Default|GetCubeTrails))
  (bind _returnvalue (* _currentlaunchdirection -1.0))
  ;[0.4319 1 0] ParticleStuff
  (Utilities|IsValid _cubetrails
    (:Is%20Valid
      (Components|Activation|Deactivate _cubetrails)
      (Utilities|FlowControl|DoOnce false) ; enters at Reset
    )
    (:Is%20Not%20Valid
      (Utilities|FlowControl|DoOnce false) ; enters at Reset
    )))

(event Custom|ControlEmitter
  (params (SpeedRate :type Float%20%28single-precision%29) (SpawnRate :type Float%20%28single-precision%29))
  (bind _cubetrails (Variables|Default|GetCubeTrails))
  ;[0.4319 1 0] ParticleStuff
  (Utilities|IsValid _cubetrails
    (:Is%20Valid
      (Effects|Components|ParticleSystem|SetFloatParameter _cubetrails "EmitterMin" (* SpeedRate (Variables|Default|GetBaseTrailSpeedMin)))
      (Effects|Components|ParticleSystem|SetFloatParameter _cubetrails "EmitterMax" (* SpeedRate (Variables|Default|GetBaseTrailSpeedMax)))
      (Effects|Components|ParticleSystem|SetFloatParameter _cubetrails "EmitterSpawnRate" (* (Variables|Default|GetBaseTrailSpawnRate) SpawnRate))
      (CallFunction|SetCubeIntensity SpawnRate))))

(event Custom|ShowBeam
  (params (BeamToLocation :type Vector))
  ;[1 1 1] BeamParticleStuff
  (if (> (Math|Vector|VectorLength (Class|Pawn|GetLastMovementInputVector)) 0.1)
    (Effects|Components|ParticleSystem|SetVectorParameter (Variables|Default|GetCubeBeam) "BeamEnd" BeamToLocation)
    (Utilities|FlowControl|DoOnce false :!label _label
      (:Completed
        (Components|Activation|Activate (Variables|Default|GetCubeBeam) false)
        (goto _label_2 Reset)))
    (else
      (Utilities|FlowControl|Sequence
        (:then_0
          (goto _label Reset))
        (:then_1
          (Utilities|FlowControl|DoOnce false :!label _label_2
            (:Completed
              (Components|Activation|Deactivate (Variables|Default|GetCubeBeam)))))))))

(event Custom|SetCubeIntensity
  (params (inIntensity :type Float%20%28single-precision%29))
  ;[0.4319 1 0] ParticleStuff
)

(event Custom|SetCollisionObjectType
  (params (LaunchedCollision :type Boolean))
  (bind _cube (Variables|Default|GetCube))
  ;[1 1 1] LaunchFunctionality, TODO: Lots of hard-coding, needs to be fixed
  (if LaunchedCollision
    (Collision|SetCollisionObjectType _cube "ECC_Vehicle")
    (else
      (Collision|SetCollisionObjectType _cube "ECC_WorldDynamic"))))

(event Custom|ResetLaunchDoOnce
  ;[1 1 1] LaunchFunctionality, TODO: Lots of hard-coding, needs to be fixed
  (Utilities|FlowControl|DoOnce false) ; enters at Reset
)

(event Custom|MoveCube
  ;[1 0 0.06404] CubeLaunch
  (if (Variables|Default|GetbCubeLaunched)
    (CallFunction|ResetCheckforCubeVelocity)
    (Class|PawnMovementComponent|AddInputVector (Variables|Default|GetFloatingPawnMovement) (* (* (Variables|Default|GetCurrentLaunchDirection) (Variables|Default|GetBaseLaunchVelocity)) (Variables|Default|GetDeltaSeconds)) true)
    (Utilities|FlowControl|DoOnce false :!label _label
      (:Completed
        (Utilities|FlowControl|Delay 0.1)
        (Variables|Default|SetbReadyToCheckCubeVelocity true)))
    (else
      (Utilities|FlowControl|DoOnce false
        (:Completed
          (Variables|Default|SetbReadyToCheckCubeVelocity false)
          (goto _label Reset))))))

(event Custom|CheckForBoundaryHit
  (bind _launchedbycharacter (Variables|Default|GetLaunchedByCharacter))
  ;[1 0 0.06404] CubeLaunch
  (if (Variables|Default|GetbReadyToCheckCubeVelocity)
    (bind _returnvalue (Physics|GetPhysicsLinearVelocity (Variables|Default|GetCube) "None"))
    (if (not (> (Math|Vector|VectorLength _returnvalue) 0.0))
      (Variables|Default|SetbCubeLaunched false)
      (Utilities|IsValid _launchedbycharacter
        (:Is%20Valid
          (if (Variables|/Game/UnsortedArtistAssets/Blueprints/BP_PlayerCharacter.BP_PlayerCharacter_C|GetbMagnetStarted _launchedbycharacter)
            (Default|MagnetEnded (Variables|Default|GetLaunchedByCharacter))
            (Variables|Default|SetbCubeAboveThresholdSpeed false))))
      (else
        (Variables|Default|SetbCubeAboveThresholdSpeed true)))))

(event EventTick
  (params (DeltaSeconds :type Float%20%28single-precision%29))
  ;[1 1 1] LaunchFunctionality, TODO: Lots of hard-coding, needs to be fixed
  (CallFunction|AddDownWardForce DeltaSeconds)
  (Variables|Default|SetDeltaSeconds DeltaSeconds)
  (CallFunction|MoveCube)
  (CallFunction|CheckforBoundaryHit)
  (if (Variables|Default|GetbCubeAboveThresholdSpeed)
    (Utilities|FlowControl|DoOnce false :!label _label
      (:Completed
        (for _array_element (Collision|GetOverlappingActors (Variables|Default|GetCubeCollision) "/Game/UnsortedArtistAssets/Blueprints/AI/BP_EnemySlow.BP_EnemySlow_C" :!class /Script/Engine.PrimitiveComponent)
          (bind _asbp_enemy_slow (Utilities|Casting|CastToBP_EnemySlow _array_element)
            (:then
              (Default|AttackReceived _asbp_enemy_slow))
            (:CastFailed
              (CallFunction|ResetLaunchDoOnce))))
        (CallFunction|ResetLaunchDoOnce)))
    (else
      (Utilities|FlowControl|DoOnce false
        (:Completed
          (CallFunction|SetCollisionObjectType false)
          (goto _label Reset))))))

(event EventBeginPlay
  (Variables|Default|SetInitialLocation (Transformation|GetActorTransform)))

(fn ConstructionScript)

(fn FindNearestDirection
  (params (X :type Float%20%28single-precision%29) (Y :type Float%20%28single-precision%29))
  (bind _output_get (LocalVariables|SettempX X))
  (bind _output_get_2 (LocalVariables|SettempY Y))
  (if (or (== (Math|Float|Round _output_get) 0) (== (Math|Float|Round _output_get_2) 0))
    (return (Math|Float|Round _output_get) (Math|Float|Round _output_get_2))
    (else
      (if (< (LocalVariables|GettempX) 0.0)
        (LocalVariables|SettempXlength (* (LocalVariables|GettempX) -1.0))
        (LocalVariables|SetxNegative true)
        (else
          (LocalVariables|SettempXlength (LocalVariables|GettempX))))
      (if (< (LocalVariables|GettempY) 0.0)
        (LocalVariables|SettempYlength (* (LocalVariables|GettempYlength) -1.0))
        (LocalVariables|SetyNegative true)
        (else
          (LocalVariables|SettempYlength (LocalVariables|GettempY))))
      (if (> (LocalVariables|GettempXlength) (LocalVariables|GettempYlength))
        (return (select (LocalVariables|GetxNegative) -1 1) 0)
        (else
          (return 0 (select (LocalVariables|GetyNegative) -1 1)))))))