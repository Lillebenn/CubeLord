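; BP_LevelTile is a level tile actor that switches on an above-ground collision volume while a player character stands on it.
; An external ActivateCollisionForTile call stores the character, shows the volume and makes it block the WorldDynamic and Vehicle channels.
; When the last overlapping player character exits, the tile hides the volume, ignores those channels, calls LeftPreviousTile on the stored character and clears the reference.
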(event OnComponentBeginOverlap(AboveGroundCollision)
  (params (OverlappedComponent :type Primitive%20Component%20Object%20Reference) (OtherActor :type Actor%20Object%20Reference) (OtherComp :type Primitive%20Component%20Object%20Reference) (OtherBodyIndex :type Integer) (bFromSweep :type Boolean) (SweepResult :type Hit%20Result%20Structure%20%28by%20ref%29)))

(event OnComponentEndOverlap(AboveGroundCollision)
  (params (OverlappedComponent :type Primitive%20Component%20Object%20Reference) (OtherActor :type Actor%20Object%20Reference) (OtherComp :type Primitive%20Component%20Object%20Reference) (OtherBodyIndex :type Integer))
  (Utilities|IsValid (Variables|Default|GetCurrentCharacterStandingOnTile)
    (:Is%20Valid
      (Utilities|Casting|CastToBP_PlayerCharacter OtherActor)
      (if (not (> (Utilities|Array|Length (Collision|GetOverlappingActors (Variables|Default|GetAboveGroundCollision) "/Game/UnsortedArtistAssets/Blueprints/BP_PlayerCharacter.BP_PlayerCharacter_C" :!class /Script/Engine.PrimitiveComponent)) 0))
        (Rendering|SetVisibility (Variables|Default|GetAboveGroundCollision) false false)
        (Collision|SetCollisionResponsetoChannel (Variables|Default|GetAboveGroundCollision) "ECC_WorldDynamic" "ECR_Ignore")
        (Collision|SetCollisionResponsetoChannel (Variables|Default|GetAboveGroundCollision) "ECC_Vehicle" "ECR_Ignore")
        (Default|LeftPreviousTile (Variables|Default|GetCurrentCharacterStandingOnTile))
        (Variables|Default|SetCurrentCharacterStandingOnTile (Variables|Default|GetEmptyPlayerCharacterVariable))))))

(event Custom|ActivateCollisionForTile
  (params (currentTouchedCharacter :type BP%20Player%20Character%20Object%20Reference))
  (Variables|Default|SetCurrentCharacterStandingOnTile currentTouchedCharacter)
  (Rendering|SetVisibility (Variables|Default|GetAboveGroundCollision) true false)
  (Collision|SetCollisionResponsetoChannel (Variables|Default|GetAboveGroundCollision) "ECC_WorldDynamic" "ECR_Block")
  (Collision|SetCollisionResponsetoChannel (Variables|Default|GetAboveGroundCollision) "ECC_Vehicle" "ECR_Block"))

(event EventBeginPlay)

(event Collision|EventActorBeginOverlap
  (params (OtherActor :type Actor%20Object%20Reference)))

(event EventTick
  (params (DeltaSeconds :type Float%20%28single-precision%29)))

(fn ConstructionScript)