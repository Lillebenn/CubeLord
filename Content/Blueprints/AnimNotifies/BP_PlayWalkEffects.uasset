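; Anim notify that plays footstep particles and sounds at a mesh socket during walk animations.
; A short line trace from the socket to 50 units above it must hit a BP_LevelTile, otherwise nothing plays.
; The tile's FloorMaterial (stone, carpet or wood) picks one of two random attenuated sounds.
; The particle is a random choice of wood or stone, independent of the floor material.
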(fn ReceivedNotify
  (params (MeshComp :type Skeletal%20Mesh%20Component%20Object%20Reference) (Animation :type Anim%20Sequence%20Base%20Object%20Reference))
  (bind _in_socket_name (Variables|Default|GetIn%20Socket%20Name))
  (bind _soundlist (Variables|Default|GetSoundList))
  (bind _returnvalue (Transformation|GetSocketLocation MeshComp _in_socket_name))
  (bind _returnvalue_2 (Transformation|GetSocketTransform MeshComp _in_socket_name "RTS_World"))
  (bind _outhit (Collision|LineTraceForObjects _returnvalue (+ _returnvalue "0, 0,50.000000") (Variables|Default|GetObject%20Types) false 0 "None"))
  (bind _asbp_level_tile (Utilities|Casting|CastToBP_LevelTile (.hitactor _outhit)))
  (Effects|SpawnEmitteratLocation (select (Math|Random|RandomBool) "/Game/Effects/Particle_Wood.Particle_Wood" "/Game/Effects/Particle_Stone.Particle_Stone") (.location _returnvalue_2) (.rotation _returnvalue_2))
  (Audio|SpawnSoundatLocation (Utilities|Select :Index (Variables|/Game/Blueprints/BP_LevelTile.BP_LevelTile_C|GetFloorMaterial _asbp_level_tile) :NewEnumerator0 (select (Math|Random|RandomBool) (Utilities|Array|Get(acopy) _soundlist 1) (Utilities|Array|Get(acopy) _soundlist)) :NewEnumerator1 (select (Math|Random|RandomBool) (Utilities|Array|Get(acopy) _soundlist 3) (Utilities|Array|Get(acopy) _soundlist 2)) :NewEnumerator2 (select (Math|Random|RandomBool) (Utilities|Array|Get(acopy) _soundlist 5) (Utilities|Array|Get(acopy) _soundlist 4))) _returnvalue "0, 0, 0" 4e+01 1.0 0.0 "/Game/Audio/BasicAttenuation.BasicAttenuation" 0)
  (return true))