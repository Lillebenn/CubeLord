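; Game instance for Puzzle Mansion that tracks Steam level achievements in the AchievementsGotten array.
; On load it caches the platform achievements and marks entries with 100 or more progress as earned.
; Handling a level achievement marks entries matching that level, writes the achievement, then after a short delay checks the totals.
; When every entry is earned, it also writes the all-levels master achievement.
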(event Custom|CheckIfHave_AllAchievements
  ;[1 1 1] check if have ALL (level) achievements
  (Variables|Default|SetAchievementsEarned 0)
  (for _array_element (Variables|Default|GetAchievementsGotten)
    (if (.isAchievementEarned (Utilities|Struct|BreakStruct_Achievements_Earned _array_element))
      (Variables|Default|SetAchievementsEarned (+ (Variables|Default|GetAchievementsEarned) 1))))
  ;;[1 1 1] if has all achievements
  (if (== (Utilities|Array|Length (Variables|Default|GetAchievementsGotten)) (Variables|Default|GetAchievementsEarned))
    (|WriteAchievementProgress (Game|GetPlayerController 0) "ACH_ALL_LEVELS_MASTER" 1e+02)))

(event Custom|loadAchivementDataFromSteam
  ;[0 1 0.03638] load in achievement data from steam - called from GameMode beginPlay
  (|CacheAchievements (Game|GetPlayerController 0)
    (:OnSuccess
      (for (_array_element _array_index) (Variables|Default|GetAchievementsGotten)
        (bind _progress (Class|AchievementBlueprintLibrary|GetCachedAchievementProgress (Game|GetPlayerController 0) (.achievementID (Utilities|Struct|BreakStruct_Achievements_Earned _array_element))))
        (Utilities|Array|SetArrayElem (Variables|Default|GetAchievementsGotten) _array_index (Utilities|Struct|MakeStruct_Achievements_Earned (>= _progress 1e+02) (.LevelName (Utilities|Struct|BreakStruct_Achievements_Earned _array_element)) (.achievementID (Utilities|Struct|BreakStruct_Achievements_Earned _array_element))))))))

(event Custom|handle_LevelAchievement
  (params (AchievementName :type Name) (CurrentLevelName :type String))
  ;[1 1 1] if you have required moves for level achievement
  (Utilities|FlowControl|Sequence
    (:then_0
      (for (_array_element _array_index) (Variables|Default|GetAchievementsGotten)
        (if (Utilities|Enum|Equal(Enum) (.LevelName (Utilities|Struct|BreakStruct_Achievements_Earned _array_element)) CurrentLevelName)
          (Utilities|Array|SetArrayElem (Variables|Default|GetAchievementsGotten) _array_index (Utilities|Struct|MakeStruct_Achievements_Earned true (.LevelName (Utilities|Struct|BreakStruct_Achievements_Earned _array_element)) (.achievementID (Utilities|Struct|BreakStruct_Achievements_Earned _array_element)))))))
    (:then_1
      (|WriteAchievementProgress (Game|GetPlayerController 0) AchievementName 1e+02))
    (:then_2
      (Utilities|FlowControl|Delay 0.2)
      (CallFunction|CheckifHaveAllAchievements))))