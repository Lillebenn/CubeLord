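; BP_CubeLordGameMode is a game mode that handles startup, audio volume settings and the pause menu.
; BeginPlay calls SetupGame, then reads Music, Master and Effects volumes from BP_PuzzleMansionGameInstance and applies them as class overrides on a base sound mix.
; The PauseGameMenu event creates and shows WBP_PauseMenu when pausing and removes it from the viewport otherwise.
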(event EventBeginPlay
  (Class|CubeLordGameMode|SetupGame)
  (bind _asbp_puzzle_mansion_game_instance (Utilities|Casting|CastToBP_PuzzleMansionGameInstance (Game|GetGameInstance)))
  (Class|GameplayStatics|SetBaseSoundMix "/Game/Audio/SoundMix.SoundMix")
  (Audio|SetSoundMixClassOverride "/Game/Audio/SoundMix.SoundMix" "/Game/Audio/Sound_Classes/Music.Music" (Variables|/Script/CubeLord.PuzzleMansionGameInstance|GetMusicVolume _asbp_puzzle_mansion_game_instance) 1.0 1.0 true)
  (Audio|SetSoundMixClassOverride "/Game/Audio/SoundMix.SoundMix" "/Game/Audio/Sound_Classes/MASTER.MASTER" (Variables|/Script/CubeLord.PuzzleMansionGameInstance|GetMasterVolume _asbp_puzzle_mansion_game_instance) 1.0 1.0 true)
  (Audio|SetSoundMixClassOverride "/Game/Audio/SoundMix.SoundMix" "/Game/Audio/Sound_Classes/Effects.Effects" (Variables|/Script/CubeLord.PuzzleMansionGameInstance|GetEffectsVolume _asbp_puzzle_mansion_game_instance) 1.0 1.0 true))

(event EventPauseGameMenu
  (params (GamePause :type Boolean))
  ;[1 1 1] create pause menu
  (if GamePause
    (bind _returnvalue (UserInterface|CreateWidget "/Game/Blueprints/Widgets/WBP_PauseMenu.WBP_PauseMenu_C"))
    (UserInterface|Viewport|AddtoViewport _returnvalue 0)
    (else
      (Widget|RemovefromParent _returnvalue))))

(fn ConstructionScript)