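; Albert is the player character, wielding a hammer that swings and magnetically pulls cube pawns.
; Right mouse locks movement and loops magnet audio while events spawn and clear a Niagara beam, whose endpoint Tick pins to the hammer head.
; Left mouse plays the swing montage, with events toggling the attack hitbox.
; CubeVolume overlaps mark the current cube; BeginPlay adds the move counter, and death disables input and shows Game Over.
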(event OnComponentBeginOverlap(CubeVolume)
  (params (OverlappedComponent :type Primitive%20Component%20Object%20Reference) (OtherActor :type Actor%20Object%20Reference) (OtherComp :type Primitive%20Component%20Object%20Reference) (OtherBodyIndex :type Integer) (bFromSweep :type Boolean) (SweepResult :type Hit%20Result%20Structure%20%28by%20ref%29))
  ;[1 1 1] on begin/end CubeVolume overlap
  (bind _asbp_cube_pawn (Utilities|Casting|CastToBP_CubePawn OtherActor))
  (Utilities|IsValid (Variables|Default|GetCurrentOverlappingCubePawn)
    (:Is%20Valid
      (bind _asbp_cube_pawn_2 (Utilities|Casting|CastToBP_CubePawn (Variables|Default|GetCurrentOverlappingCubePawn)))
      (Default|EndCurrent _asbp_cube_pawn_2))
    (:Is%20Not%20Valid
      _))
  (Default|SetCurrent _asbp_cube_pawn)
  (Variables|Default|SetCurrentOverlappingCubePawn _asbp_cube_pawn))

(event OnComponentEndOverlap(CubeVolume)
  (params (OverlappedComponent :type Primitive%20Component%20Object%20Reference) (OtherActor :type Actor%20Object%20Reference) (OtherComp :type Primitive%20Component%20Object%20Reference) (OtherBodyIndex :type Integer))
  ;[1 1 1] on begin/end CubeVolume overlap
  (bind _asbp_cube_pawn (Utilities|Casting|CastToBP_CubePawn OtherActor))
  (Default|EndCurrent _asbp_cube_pawn)
  (bind _array_element (Utilities|Array|ForEachLoopwithBreak (Collision|GetOverlappingActors (Variables|Default|GetCubeVolume) 0 :!class /Script/Engine.PrimitiveComponent))
    (:LoopBody
      (bind _asbp_cube_pawn_2 (Utilities|Casting|CastToBP_CubePawn _array_element))
      (CallFunction|BreakSearchLoop)
      (Utilities|IsValid (Variables|Default|GetCurrentOverlappingCubePawn)
        (:Is%20Valid
          (bind _asbp_cube_pawn_3 (Utilities|Casting|CastToBP_CubePawn (Variables|Default|GetCurrentOverlappingCubePawn)))
          (Default|EndCurrent _asbp_cube_pawn_3)
          (Default|SetCurrent _asbp_cube_pawn_2)
          (Variables|Default|SetCurrentOverlappingCubePawn _asbp_cube_pawn_2))))))

(event Custom|ActionEnd
  ;[1 1 1] set walkspeed on action start/end
  (Variables|/Script/Engine.CharacterMovementComponent|SetMaxWalkSpeed (Variables|Character|GetCharacterMovement) 8e+02))

(event Custom|HitboxDeactivate
  ;[1 1 1] hitbox de/activate
  (Class|AlbertCharacter|StopAttacking))

(event Custom|AlbertDeath
  (bind _returnvalue (Game|GetPlayerController 0))
  ;[0 0 0] Death
  (Variables|Default|SetbIsPulling false)
  (Variables|Default|SetbDeath true)
  (Input|DisableInput (Game|Player|GetPlayerPawn 0) (Game|GetPlayerController 0))
  (Utilities|FlowControl|Delay 0.2)
  (Audio|PlaySoundatLocation "/Game/Audio/Temp/DEATH.DEATH" (Transformation|GetSocketLocation (Variables|Character|GetMesh) "BoneSocket") "0, 0, 0" 1.0 1.0 0.0 "/Game/Audio/BasicAttenuation.BasicAttenuation" 0 0)
  (Utilities|FlowControl|Delay 1.0)
  (Variables|/Script/Engine.PlayerController|SetbShowMouseCursor _returnvalue true)
  (bind _returnvalue_2 (UserInterface|CreateWidget "/Game/Blueprints/Widgets/WBP_GameOver.WBP_GameOver_C" _returnvalue))
  (UserInterface|Viewport|AddtoViewport _returnvalue_2 0))

(event Custom|ActionStart
  ;[1 1 1] set walkspeed on action start/end
  (Variables|/Script/Engine.CharacterMovementComponent|SetMaxWalkSpeed (Variables|Character|GetCharacterMovement) 0.0))

(event Custom|BreakSearchLoop
  ;[1 1 1] on begin/end CubeVolume overlap
  (Utilities|Array|ForEachLoopwithBreak (Collision|GetOverlappingActors (Variables|Default|GetCubeVolume) 0 :!class /Script/Engine.PrimitiveComponent)) ; enters at Break
)

(event Custom|HitboxActivate
  ;[1 1 1] hitbox de/activate
  (Class|AlbertCharacter|StartAttacking))

(event EventSpawnHammerHitFX
  (params (Transform :type Transform))
  ;[1 1 1] spawn hammer hit FX
  (Niagara|SpawnSystematLocation "/Game/Effects/NS_CubeHit.NS_CubeHit" (Transformation|GetSocketLocation (Variables|Default|GetHammer) "HammerHead") (.rotation Transform) (.scale Transform)))

(event EventTick
  (params (DeltaSeconds :type Float%20%28single-precision%29))
  (bind _ns_cubeelectricfield (Variables|Default|GetNS_CubeElectricField))
  ;[1 0.8703 0] tick - hammer beak and set magnetic cube detected
  (Utilities|FlowControl|Sequence
    (:then_0
      (bind _currenttraileffects (Variables|Default|GetCurrentTrailEffects)
        (:then
          (Effects|Components|ParticleSystem|SetVectorParameter _currenttraileffects "BeamEnd" (Transformation|GetSocketLocation (Variables|Default|GetHammerMesh) "HammerHead")))
        (:else)))
    (:then_1
      (if (Variables|Default|GetbMagneticCubeDetected)
        (Effects|Components|ParticleSystem|SetFloatParameter _ns_cubeelectricfield "Rate" 5e+01)
        (else
          (Effects|Components|ParticleSystem|SetFloatParameter _ns_cubeelectricfield "Rate" 0.0))))))

(event EventEventStopHammerPullBlueprint
  (params (Delay :type Float%20%28single-precision%29))
  (bind _charactermovement (Variables|Character|GetCharacterMovement))
  ;[1 0.8446 0] Magnet
  (Utilities|FlowControl|Delay Delay)
  (Variables|Default|SetbIsPulling false)
  (Variables|/Script/Engine.CharacterMovementComponent|SetMaxWalkSpeed _charactermovement (Variables|Default|GetDefaultMaxWalkSpeed))
  (Variables|/Script/Engine.CharacterMovementComponent|SetRotationRate _charactermovement (Math|Rotator|MakeRotator 0.0 0.0 (Variables|Default|GetDefaultRotationRate)))
  (bind _currenttraileffects (Variables|Default|GetCurrentTrailEffects)
    (:then
      (Components|DestroyComponent _currenttraileffects))
    (:else)))

(event EventCallDeath
  (bind _returnvalue (Game|GetPlayerController 0))
  ;[0 0 0] Death
  (Variables|Default|SetbIsPulling false)
  (Variables|Default|SetbDeath true)
  (Input|DisableInput (Game|Player|GetPlayerPawn 0) (Game|GetPlayerController 0))
  (Utilities|FlowControl|Delay 0.2)
  (Audio|PlaySoundatLocation "/Game/Audio/Temp/DEATH.DEATH" (Transformation|GetSocketLocation (Variables|Character|GetMesh) "BoneSocket") "0, 0, 0" 1.0 1.0 0.0 "/Game/Audio/BasicAttenuation.BasicAttenuation" 0 0)
  (Utilities|FlowControl|Delay 1.0)
  (Variables|/Script/Engine.PlayerController|SetbShowMouseCursor _returnvalue true)
  (bind _returnvalue_2 (UserInterface|CreateWidget "/Game/Blueprints/Widgets/WBP_GameOver.WBP_GameOver_C" _returnvalue))
  (UserInterface|Viewport|AddtoViewport _returnvalue_2 0))

(event EventEventSpawnMagneticPullFX
  (params (InCubeHit :type Actor%20Object%20Reference))
  ;[1 0.8446 0] Magnet
  (bind _asbp_cube_pawn (Utilities|Casting|CastToBP_CubePawn InCubeHit))
  (Utilities|IsValid (Variables|/Script/CubeLord.CubePawn|GetCubeMesh _asbp_cube_pawn)
    (:Is%20Valid
      (bind _returnvalue (Niagara|SpawnSystemAttached "/Game/UnsortedArtistAssets/Particles/NS_CubeBeam.NS_CubeBeam" (Variables|/Script/CubeLord.CubePawn|GetCubeMesh _asbp_cube_pawn) "CubeCenter" (Transformation|GetSocketLocation (Variables|/Script/CubeLord.CubePawn|GetCubeMesh _asbp_cube_pawn) "CubeCenter") "0, 0, 0" "KeepWorldPosition" false))
      (Effects|Components|ParticleSystem|SetVectorParameter _returnvalue "BeamEnd" (Transformation|GetSocketLocation (Variables|Default|GetHammerMesh) "HammerHead"))
      (Components|Activation|Activate _returnvalue false)
      (Variables|Default|SetCurrentTrailEffects _returnvalue))))

(event EventBeginPlay
  ;[1 1 1] add move counter to viewport
  (bind _returnvalue (UserInterface|CreateWidget "/Game/Blueprints/Widgets/WBP_MoveCounter.WBP_MoveCounter_C"))
  (UserInterface|Viewport|AddtoViewport _returnvalue 0))

(event Input|MouseEvents|LeftMouseButton
  (params (Key :type Key%20Structure :default "None"))
  ;[1 1 1] left mouse button - play anim swing
  (:Pressed
    (Animation|PlayAnimMontage "/Game/Meshes/Characters/Albert/HammerSwing_Montage.HammerSwing_Montage" 1.0 "None")))

(event Input|MouseEvents|RightMouseButton
  (params (Key :type Key%20Structure :default "None"))
  ;[1 0.8446 0] Magnet
  (:Pressed
    (if (Variables|Default|GetbIsNotDiagonal)
      (Variables|Default|SetbIsPulling true)
      (Variables|/Script/Engine.CharacterMovementComponent|SetMaxWalkSpeed (Variables|Character|GetCharacterMovement) 0.0)
      (Variables|/Script/Engine.CharacterMovementComponent|SetRotationRate (Variables|Character|GetCharacterMovement) (Math|Rotator|MakeRotator 0.0 0.0 0.0))
      (Audio|PlaySoundatLocation "/Game/Audio/S_MagnetStart.S_MagnetStart" (Transformation|GetSocketLocation (Variables|Default|GetCapsuleComponent) "HammerHead") "0, 0, 0" 1.0 1.0 0.0 "/Game/Audio/BasicAttenuation.BasicAttenuation" 0 0)
      (Utilities|FlowControl|Delay 0.1)
      (bind _newtrack_0 (Timeline|PitchChange Play)
        (:Update
          (if (and (Game|Player|IsInputKeyDown (Game|GetPlayerController 0) "RightMouseButton") (Variables|Default|GetbIsPulling))
            (Audio|PlaySoundatLocation "/Game/Audio/S_MagnetStart.S_MagnetStart" (Transformation|GetSocketLocation (Variables|Default|GetCapsuleComponent) "HammerHead") "0, 0, 0" 0.1 _newtrack_0 0.0 "/Game/Audio/BasicAttenuation.BasicAttenuation" 0 0 :!label _label)
            (Utilities|FlowControl|Delay 1.0)
            (if (Variables|Default|GetbIsPulling)
              (goto _label))))))))

(fn ConstructionScript)