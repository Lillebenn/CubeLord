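; Blueprint that unlocks the ACH_STRIKE achievement when four enemies are taken down at nearly the same time.
; The first OnEnemyHit call starts a half-second Delay, and every call increments a shared counter.
; After the delay, a count of four or more writes achievement progress for player controller 0.
; The timer flag and counter are never reset here, so only the first hit opens a window.
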(event Custom|OnEnemyHit
  ;[1 1 1] unlock achievement by taking down all 4 enemies at the same time
  (if (Variables|Default|GetTimerStarted)
    ;;[1 1 1] only count
    (Variables|Default|SetEnemyCounter (+ (Variables|Default|GetEnemyCounter) 1))
    (else
      (Variables|Default|SetTimerStarted true)
      (Variables|Default|SetEnemyCounter (+ (Variables|Default|GetEnemyCounter) 1))
      (Utilities|FlowControl|Delay 0.5)
      (if (>= (Variables|Default|GetEnemyCounter) 4)
        (|WriteAchievementProgress (Game|GetPlayerController 0) "ACH_STRIKE" 1e+02)))))

(fn ConstructionScript)