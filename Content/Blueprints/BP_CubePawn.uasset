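; BP_CubePawn is a stone cube pawn with hit sounds, a motion trail and a light indicator switched on and off as current.
; PlaySound briefly raises a recent-hit counter and plays a hammer-rock sound, suppressed for non-magnetic cubes while BP_Albert is pulling.
; While that counter is positive, Tick drives the Niagara trail's spawn rate and reversed direction from the mesh's physics velocity.
; A separate event plays a stone-block stop sound.
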(event Custom|SetCurrent
  ;[1 1 1] Glowing on/off
  (Rendering|Components|Light|SetIntensity (Variables|Default|GetLightIndicator) 5e+03))

(event Custom|EndCurrent
  ;[1 1 1] Glowing on/off
  (Rendering|Components|Light|SetIntensity (Variables|Default|GetLightIndicator) 0.0))

(event Custom|SetParticleSpawning
  (bind _cubemesh (Variables|Default|GetCubeMesh))
  ;[1 0.4828 0.9627] called on tick
  (Utilities|FlowControl|Sequence
    (:then_0
      (bind _returnvalue (Physics|GetPhysicsLinearVelocity _cubemesh "None"))
      (if (> (Math|Vector|VectorLength _returnvalue) 1.0)
        (Effects|Components|ParticleSystem|SetFloatParameter (Variables|Default|GetCubeTrails) "InSpawnRate" (* (Math|Vector|VectorLength _returnvalue) 0.3))
        (else
          (Effects|Components|ParticleSystem|SetFloatParameter (Variables|Default|GetCubeTrails) "InSpawnRate" 0.0))))
    (:then_1
      (bind _returnvalue_2 (Physics|GetPhysicsLinearVelocity _cubemesh "None"))
      (Effects|Components|ParticleSystem|SetVectorParameter (Variables|Default|GetCubeTrails) "InVectorDirection" (* (* _returnvalue_2 -0.3) "1.000000,1.000000,5.000000")))))

(event EventBeginPlay
  ;[1 1 1] beginPlay
  (Class|NiagaraFunctionLibrary|OverrideSystemUserVariableStaticMeshComponent (Variables|Default|GetCubeTrails) "InMesh" (Variables|Default|GetCubeMesh)))

(event EventPlaySoundatStop
  ;[1 1 1] play sound
  (Audio|PlaySoundatLocation "/Game/Audio/Cube/S_StoneblockStop.S_StoneblockStop" (Transformation|GetActorLocation) "0, 0, 0" 5.0 1.0 0.0 "/Game/Audio/BasicAttenuation.BasicAttenuation" 0 0))

(event EventTick
  (params (DeltaSeconds :type Float%20%28single-precision%29))
  ;[1 0.4012 0.801] on Tick
  ;[1 1 1] (could be) Used to check if particles should be spawned
  (if (> (Variables|Default|GettimesHitLately) 0)
    (CallFunction|SetParticleSpawning)))

(event EventPlaySound
  ;[1 1 1] play sound
  (Utilities|FlowControl|Sequence
    (:then_0
      ;[1 1 1] (could be) Used to check if particles should be spawned
      (bind _output_get (Variables|Default|SettimesHitLately (+ (stale _output_get) 1)))
      (Utilities|FlowControl|Delay 2.0)
      (bind _output_get_2 (Variables|Default|SettimesHitLately (- (stale _output_get_2) 1))))
    (:then_1
      (if (not (Variables|Default|GetbIsMagnetic))
        (bind _asbp_albert (Utilities|Casting|CastToBP_Albert (Game|Player|GetPlayerPawn 0)))
        (Utilities|IsValid _asbp_albert
          (:Is%20Valid
            (if (not (Variables|/Script/CubeLord.Albert_Character|GetbIsPulling _asbp_albert))
              (Audio|PlaySoundatLocation "/Game/Audio/Cube/Soundly/HammerRock.HammerRock" (Transformation|GetActorLocation) "0, 0, 0" 5.0 1.0 0.0 "/Game/Audio/BasicAttenuation.BasicAttenuation" 0 0 :!label _label))))
        (else
          (goto _label))))))

(fn ConstructionScript)

(fn SetParticleSpawnRate)