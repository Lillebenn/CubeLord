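; BP_MusicPlayer is an actor that plays a music intro followed by a separate loop track.
; BeginPlay starts the intro, waits through a Delay equal to the sound's duration, then starts the loop; older playback-percent triggers remain unused.
; It disables tick-when-paused on both audio components but enables it on the actor.
; Stop halts and deactivates both components, then destroys the actor.
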(event OnAudioPlaybackPercent(Music_Loop)
  (params (PlayingSoundWave :type Sound%20Wave%20Object%20Reference) (PlaybackPercent :type Float%20%28single-precision%29))
  ;[1 0 0] outdated - set loop files to looping instead
)

(event Custom|Stop
  (bind _music_intro (Variables|Default|GetMusic_Intro))
  (bind _music_loop (Variables|Default|GetMusic_Loop))
  ;[1 1 1] Stop
  (Audio|Components|Audio|Stop _music_intro)
  (Components|Activation|Deactivate _music_intro)
  (Audio|Components|Audio|Stop _music_loop)
  (Components|Activation|Deactivate _music_loop)
  (Actor|DestroyActor))

(event EventBeginPlay
  (bind _music_intro (Variables|Default|GetMusic_Intro))
  ;[1 1 1] beginPlay - set tickable & Play
  (Utilities|FlowControl|DoOnce false
    (:Completed
      (Class|ActorComponent|SetTickablewhenPaused (Variables|Default|GetMusic_Intro) false)
      (Class|ActorComponent|SetTickablewhenPaused (Variables|Default|GetMusic_Loop) false)
      (Class|Actor|SetTickablewhenPaused true)
      (Audio|Components|Audio|Play _music_intro 0.0)
      ;[1 1 1] wait until intro stops, then start loop
      (Utilities|FlowControl|Delay (Variables|/Script/Engine.SoundBase|GetDuration (Variables|/Script/Engine.AudioComponent|GetSound _music_intro)))
      (Utilities|FlowControl|DoOnce false
        (:Completed
          (Audio|Components|Audio|Play (Variables|Default|GetMusic_Loop) 0.0))))))

(fn ConstructionScript)