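; BP_Albert is the player character, a hammer wielder with a magnet pull and a montage-driven swing whose events toggle attacking.
; Holding right mouse while IsNotDiagonal roots movement, sets IsPulling and repeats a timeline-pitched magnet sound from the hammer head.
; CubeVolume overlaps mark the current BP_CubePawn, ending the previous one.
; Death events disable input and show the game-over widget, while a Testing input toggles the end-title widget.
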(event OnComponentBeginOverlap(CubeVolume)
  (params (OverlappedComponent :type Primitive%20Component%20Object%20Reference) (OtherActor :type Actor%20Object%20Reference) (OtherComp :type Primitive%20Component%20Object%20Reference) (OtherBodyIndex :type Integer) (bFromSweep :type Boolean) (SweepResult :type Hit%20Result%20Structure%20%28by%20ref%29))
  (bind _asbp_cube_pawn (Utilities|Casting|CastToBP_CubePawn OtherActor))
  (Utilities|IsValid (Variables|Default|GetCurrentOverlappingCubePawn)
    (:Is%20Valid
      (bind _asbp_cube_pawn_2 (Utilities|Casting|CastToBP_CubePawn (Variables|Default|GetCurrentOverlappingCubePawn)))
      (Default|EndCurrent _asbp_cube_pawn_2))
    (:Is%20Not%20Valid
      _))
  (Default|SetCurrent _asbp_cube_pawn)
  (Variables|Default|SetCurrentOverlappingCubePawn _asbp_cube_pawn))

(event OnComponentEndOverlap(CubeVolume)
  (params (OverlappedComponent :type Primitive%20Component%20Object%20Reference) (OtherActor :type Actor%20Object%20Reference) (OtherComp :type Primitive%20Component%20Object%20Reference) (OtherBodyIndex :type Integer))
  (bind _asbp_cube_pawn (Utilities|Casting|CastToBP_CubePawn OtherActor))
  (Default|EndCurrent _asbp_cube_pawn))

(event Custom|ActionEnd
  (Variables|/Script/Engine.CharacterMovementComponent|SetMaxWalkSpeed (Variables|Character|GetCharacterMovement) 8e+02))

(event Custom|HitboxDeactivate
  (Class|AlbertCharacter|StopAttacking))

(event Custom|SpikeDeath
  (bind _returnvalue (Game|GetPlayerController 0))
  (Input|DisableInput (Game|Player|GetPlayerPawn 0) (Game|GetPlayerController 0))
  (Utilities|FlowControl|Delay 0.2)
  (Audio|PlaySoundatLocation "/Game/Audio/Temp/DEATH.DEATH" (Transformation|GetSocketLocation (Variables|Character|GetMesh) "BoneSocket") "0, 0, 0" 1.0 1.0 0.0 "/Game/Audio/BasicAttenuation.BasicAttenuation" 0 0)
  (Utilities|FlowControl|Delay 1.0)
  (Variables|/Script/Engine.PlayerController|SetbShowMouseCursor _returnvalue true)
  (bind _returnvalue_2 (UserInterface|CreateWidget "/Game/Blueprints/Widgets/WBP_GameOver.WBP_GameOver_C" _returnvalue))
  (UserInterface|Viewport|AddtoViewport _returnvalue_2 0))

(event Custom|ActionStart
  (Variables|/Script/Engine.CharacterMovementComponent|SetMaxWalkSpeed (Variables|Character|GetCharacterMovement) 0.0))

(event Custom|HitboxActivate
  (Class|AlbertCharacter|StartAttacking))

(event EventSpawnHammerHitFX
  (params (Transform :type Transform))
  (Niagara|SpawnSystematLocation "/Game/Effects/NS_CubeHit.NS_CubeHit" (Transformation|GetSocketLocation (Variables|Default|GetHammer) "HammerHead") (.rotation Transform) (.scale Transform)))

(event EventTick
  (params (DeltaSeconds :type Float%20%28single-precision%29)))

(event EventCallDeath
  (bind _returnvalue (Game|GetPlayerController 0))
  (Variables|Default|SetbIsPulling false)
  (Input|DisableInput (Game|Player|GetPlayerPawn 0) (Game|GetPlayerController 0))
  (Utilities|FlowControl|Delay 0.2)
  (Audio|PlaySoundatLocation "/Game/Audio/Temp/DEATH.DEATH" (Transformation|GetSocketLocation (Variables|Character|GetMesh) "BoneSocket") "0, 0, 0" 1.0 1.0 0.0 "/Game/Audio/BasicAttenuation.BasicAttenuation" 0 0)
  (Utilities|FlowControl|Delay 1.0)
  (Variables|/Script/Engine.PlayerController|SetbShowMouseCursor _returnvalue true)
  (bind _returnvalue_2 (UserInterface|CreateWidget "/Game/Blueprints/Widgets/WBP_GameOver.WBP_GameOver_C" _returnvalue))
  (UserInterface|Viewport|AddtoViewport _returnvalue_2 0))

(event Input|ActionEvents|InputActionTesting
  (params (Key :type Key%20Structure :default "None"))
  (:Pressed
    (Utilities|FlowControl|FlipFlop
      (:A
        (bind _returnvalue (UserInterface|CreateWidget "/Game/Blueprints/Widgets/WBP_EndTitle.WBP_EndTitle_C"))
        (UserInterface|Viewport|AddtoViewport _returnvalue 0))
      (:B
        (Widget|RemovefromParent _returnvalue)))))

(event Input|MouseEvents|LeftMouseButton
  (params (Key :type Key%20Structure :default "None"))
  (:Pressed
    (Animation|PlayAnimMontage "/Game/Meshes/Characters/Albert/HammerSwing_Montage.HammerSwing_Montage" 1.0 "None")))

(event Input|MouseEvents|RightMouseButton
  (params (Key :type Key%20Structure :default "None"))
  (bind _charactermovement (Variables|Character|GetCharacterMovement))
  (:Pressed
    (if (Variables|Default|GetbIsNotDiagonal)
      (Variables|Default|SetbIsPulling true)
      (Variables|/Script/Engine.CharacterMovementComponent|SetMaxWalkSpeed _charactermovement 0.0)
      (Audio|PlaySoundatLocation "/Game/Audio/S_MagnetStart.S_MagnetStart" (Transformation|GetSocketLocation (Variables|Default|GetCapsuleComponent) "HammerHead") "0, 0, 0" 1.0 1.0 0.0 "/Game/Audio/BasicAttenuation.BasicAttenuation" 0 0)
      (Utilities|FlowControl|Delay 0.1)
      (bind _newtrack_0 (Timeline|PitchChange Play)
        (:Update
          (if (and (Game|Player|IsInputKeyDown (Game|GetPlayerController 0) "RightMouseButton") (Variables|Default|GetbIsPulling))
            (Audio|PlaySoundatLocation "/Game/Audio/S_MagnetStart.S_MagnetStart" (Transformation|GetSocketLocation (Variables|Default|GetCapsuleComponent) "HammerHead") "0, 0, 0" 0.1 _newtrack_0 0.0 "/Game/Audio/BasicAttenuation.BasicAttenuation" 0 0 :!label _label)
            (Utilities|FlowControl|Delay 1.0)
            (if (Variables|Default|GetbIsPulling)
              (goto _label)))))))
  (:Released
    (Variables|Default|SetbIsPulling false)
    (Variables|/Script/Engine.CharacterMovementComponent|SetMaxWalkSpeed _charactermovement 8e+02)))

(fn ConstructionScript)